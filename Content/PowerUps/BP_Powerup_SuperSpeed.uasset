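; Super speed power-up Blueprint that temporarily doubles the walk speed of the actor that activates it.
; OnActivated stores that actor as ReceivingPlayer, sets its CharacterMovementComponent MaxWalkSpeed to twice GetMaxSpeed and prints a debug string.
; OnExpired sets it to half the current GetMaxSpeed, rather than restoring a saved value, then calls the parent's expiry logic.
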(event EventOnExpired
  (bind _receivingplayer (Variables|Default|GetReceivingPlayer))
  (bind _returnvalue (Actor|GetComponentbyClass _receivingplayer "/Script/Engine.CharacterMovementComponent"))
  (Variables|/Script/Engine.CharacterMovementComponent|SetMaxWalkSpeed _returnvalue (/ (Class|MovementComponent|GetMaxSpeed _returnvalue) 2.0))
  (|CallParentFunction))

(event EventOnActivated
  (params (OtherActor :type Actor%20Object%20Reference))
  (bind _returnvalue (Actor|GetComponentbyClass OtherActor "/Script/Engine.CharacterMovementComponent"))
  (Variables|Default|SetReceivingPlayer OtherActor)
  (Variables|/Script/Engine.CharacterMovementComponent|SetMaxWalkSpeed _returnvalue (* (Class|MovementComponent|GetMaxSpeed _returnvalue) 2.0))
  (Development|PrintString "Hello"))

(fn ConstructionScript)